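; BP_Spawn_A is an enemy spawner that creates BP_AiEnemy at its own transform, then destroys itself.
; A half-second Delay on Tick throttles repeated spawning, and each enemy receives a default controller.
; An AIMoveTo targets a random reachable point near the spawner, with no pawn input shown.
; Its immediate output calls AIEnemykilld on ThirdPersonGameMode and starts a ten-second Delay before destroying the spawner.
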(event `self.ReceiveBeginPlay`)

(event `self.ReceiveTick`
  (params (DeltaSeconds :type "Float (single-precision)"))
  (`KismetSystemLibrary.Delay` 0.5)
  (bind _returnvalue (`|SpawnActorFromClass` "/Game/BluePrints/Characters/BP_AiEnemy.BP_AiEnemy_C" (`self.GetTransform`) "AdjustIfPossibleButAlwaysSpawn" "OverrideRootScale" null null))
  (`Pawn.SpawnDefaultController` _returnvalue)
  (`|AIMoveTo` null (`NavigationSystemV1.K2_GetRandomReachablePointInRadius` (`self.K2_GetActorLocation`) 500.0 null null) null
    (:`then`
      (bind _asthird_person_game_mode (cast `/Game/BluePrints/Characters/ThirdPersonGameMode` (`GameplayStatics.GetGameMode`)))
      (`/Game/BluePrints/Characters/ThirdPersonGameMode.BP_AIEnemykilld` _asthird_person_game_mode)
      (`KismetSystemLibrary.Delay` 10.0)
      (`self.K2_DestroyActor`))))

(fn `UserConstructionScript`)
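; BP_AiEnemy is an enemy character that chases the player and plays a magic attack montage on arrival.
; PawnSensing sets CanSeeEnemy and starts the AIMoveTo chase; Tick, gated by that same flag, also issues delayed random nearby moves.
; AnyDamage reduces health and, at zero, plays a death montage before destroying the actor, while overlapping a BP_Bulit destroys it immediately.
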(event `self.ReceiveActorBeginOverlap`
  (params (OtherActor :type "Actor Object Reference"))
  (cast `/Game/BluePrints/Characters/BP_Bulit` OtherActor)
  (`self.K2_DestroyActor`))

(event `self.ReceiveAnyDamage`
  (params (Damage :type "Float (single-precision)") (DamageType :type "DamageType Object Reference") (InstigatedBy :type "Controller Object Reference") (DamageCauser :type "Actor Object Reference"))
  (bind _output_get (set `self.CurrentHealth` (- (`self.CurrentHealth`) Damage)))
  (`KismetSystemLibrary.PrintString` (`KismetStringLibrary.Conv_DoubleToString` _output_get))
  (if (<= _output_get 0.0)
    (`self.PlayAnimMontage` "/Game/dd/Content/CityofBrass_Enemies/Meshes/Enemy/Charger/Animation/death_Montage.death_Montage")
    (`KismetSystemLibrary.Delay` 3.0)
    (`self.K2_DestroyActor`)))

(event `CustomEvent`
  (params (Damage :type "Float (double-precision)"))
  (bind _output_get (set `self.CurrentHealth` (- (`self.CurrentHealth`) Damage)))
  (if (<= _output_get 0.0)
    (`KismetSystemLibrary.PrintString` "EnemyDaed" true true (struct :`R` 1.0 :`G` 0.018722 :`A` 1.0))
    (else
      (`KismetSystemLibrary.PrintString` "Hello" true true (struct :`R` 0.104136 :`G` 0.030858 :`B` 1.0 :`A` 1.0)))))

(event `self.ReceiveTick`
  (params (DeltaSeconds :type "Float (single-precision)"))
  (`KismetSystemLibrary.Delay` 0.5)
  (if (`self.CanSeeEnemy?`)
    (`KismetSystemLibrary.Delay` (`KismetMathLibrary.RandomFloatInRange` 5.0 10.0))
    (`|AIMoveTo` self (`NavigationSystemV1.K2_GetRandomReachablePointInRadius` (`self.K2_GetActorLocation`) 300.0 null "/Script/AIModule.NavFilter_AIControllerDefault") null)))

(event `self.PawnSensing.OnSeePawn`
  (params (Pawn :type "Pawn Object Reference"))
  ;[1 1 1] 플레이어가 보이면 따라오기
  (set `self.CanSeeEnemy?` true)
  (`self.FollowPlayer`))

(event `FollowPlayer`
  ;[1 1 1] Ai 무브먼트 공격
  (set `self.canAttck?` true)
  (if (`self.CanSeeEnemy?`)
    (`|AIMoveTo` self (0.0 0.0 0.0) (`GameplayStatics.GetPlayerCharacter` 0) 70.0
      (:`OnSuccess`
        (if (`self.canAttck?`)
          (set `self.canAttck?` false)
          (bind _returnvalue (`self.PlayAnimMontage` "/Game/ThirdPerson/Animation/Standing_Magic_Attack_01_Anim_Montage.Standing_Magic_Attack_01_Anim_Montage"))
          (`KismetSystemLibrary.Delay` _returnvalue)
          (set `self.canAttck?` true))))
    (else
      (set `self.CanSeeEnemy?` false))))

(fn `UserConstructionScript`)
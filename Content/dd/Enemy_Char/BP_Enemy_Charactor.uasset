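; Enemy character Blueprint that tracks health and dies from damage.
; AnyDamage subtracts from CurrentHealth, prints it, and at zero or below plays a death montage, then destroys the actor after a short delay.
; A separate OverRapEnemy event also subtracts health but only prints the value or a death message, without destroying the enemy.
; UpdateWalkSpeed sets the movement component's maximum walk speed.
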(event `self.ReceiveAnyDamage`
  (params (Damage :type "Float (single-precision)") (DamageType :type "DamageType Object Reference") (InstigatedBy :type "Controller Object Reference") (DamageCauser :type "Actor Object Reference"))
  (bind _output_get (set `self.CurrentHealth` (- (`self.CurrentHealth`) Damage)))
  (`KismetSystemLibrary.PrintString` (`KismetStringLibrary.Conv_DoubleToString` _output_get))
  (if (<= _output_get 0.0)
    (`self.PlayAnimMontage` "/Game/dd/Content/CityofBrass_Enemies/Meshes/Enemy/Charger/Animation/death_Montage.death_Montage")
    (`KismetSystemLibrary.Delay` 3.0)
    (`self.K2_DestroyActor`)))

(event `/Game/dd/Enemy_Char/BP_IP_Enemy.Over Rap Enemy`
  (params (Damage :type "Float (double-precision)"))
  (bind _output_get (set `self.CurrentHealth` (- (`self.CurrentHealth`) Damage)))
  (if (<= _output_get 0.0)
    (`KismetSystemLibrary.PrintString` "EnemyDaed" true true (struct :`R` 1.0 :`G` 0.018722 :`A` 1.0))
    (else
      (`KismetSystemLibrary.PrintString` (`KismetStringLibrary.Conv_DoubleToString` _output_get) true true (struct :`R` 0.104136 :`G` 0.030858 :`B` 1.0 :`A` 1.0)))))

(fn `Update Walk Speed`
  (params (NewWalkSpeed :type "Float (double-precision)"))
  (set `CharacterMovementComponent.MaxWalkSpeed` NewWalkSpeed (`self.CharacterMovement`)))

(fn `UserConstructionScript`)